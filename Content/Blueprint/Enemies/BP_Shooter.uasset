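; BP_Shooter is an enemy character that chases the player and deals damage on contact through its capsule hit.
; PawnSensing spotting the first-person character starts an AIMoveTo toward it and sets a never-cleared flag that makes Tick yaw the enemy toward the player.
; Damage reduces its life and, if non-lethal, also sets that flag.
; At zero life, a DoOnce deactivates movement and destroys the actor after a short delay.
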(event `self.ReceiveBeginPlay`
  (set `self.Life` 50.0))

(event `self.ReceiveTick`
  (params (DeltaSeconds :type "Float (single-precision)"))
  (bind (_returnvalue_roll _returnvalue_pitch _returnvalue_yaw) (`KismetMathLibrary.BreakRotator` (`KismetMathLibrary.FindLookAtRotation` (`self.K2_GetActorLocation`) (`self.K2_GetActorLocation` (`GameplayStatics.GetPlayerCharacter` 0)))))
  (if (`self.canSeePlayer`)
    (`self.K2_SetActorRotation` (`KismetMathLibrary.MakeRotator` 0.0 0.0 _returnvalue_yaw))))

(event `self.PawnSensing.OnSeePawn`
  (params (Pawn :type "Pawn Object Reference"))
  (bind _asbp_first_person_character (cast `/Game/FirstPerson/Blueprints/BP_FirstPersonCharacter` Pawn))
  (set `self.canSeePlayer` true)
  (`|AIMoveTo` self (0.0 0.0 0.0) _asbp_first_person_character))

(event `self.ReceiveAnyDamage`
  (params (Damage :type "Float (single-precision)") (DamageType :type "DamageType Object Reference") (InstigatedBy :type "Controller Object Reference") (DamageCauser :type "Actor Object Reference"))
  (bind _output_get (set `self.Life` (- (`self.Life`) Damage)))
  (if (<= _output_get 0.0)
    (`/Engine/EditorBlueprintResources/StandardMacros.DoOnce` false
      (:`Completed`
        (`ActorComponent.Deactivate` (`self.CharacterMovement`))
        (`KismetSystemLibrary.Delay` 0.2)
        (`self.K2_DestroyActor`)))
    (else
      (set `self.canSeePlayer` true))))

(event `self.CapsuleComponent.OnComponentHit`
  (params (HitComponent :type "PrimitiveComponent Object Reference") (OtherActor :type "Actor Object Reference") (OtherComp :type "PrimitiveComponent Object Reference") (NormalImpulse :type "Vector Structure") (Hit :type "HitResult Structure (by ref)"))
  (`GameplayStatics.ApplyDamage` OtherActor (`self.damage`)))

(fn `UserConstructionScript`)