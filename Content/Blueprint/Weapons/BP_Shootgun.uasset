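; BP_Shootgun is a shotgun weapon Blueprint that handles the Shoot event.
; Shoot passes through a DoOnce, sets range and damage, calls FireWeapon, then plays the shotgun sound at the world origin.
; ResetWeapon reopens the DoOnce immediately after each shot, as the one-second Delay leading to it is unconnected, so no cooldown applies.
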(event `self.Shoot`
  (`/Engine/EditorBlueprintResources/StandardMacros.DoOnce` false :!label _label
    (:`Completed`
      (set `self.Range` 1000.0)
      (set `self.WeaponDamage` 50.0)
      (`self.FireWeapon`)
      (`GameplayStatics.PlaySoundAtLocation` "/Game/MilitaryWeapSilver/Sound/Shotgun/Wavs/ShotgunA_Fire_ST04.ShotgunA_Fire_ST04" (0.0 0.0 0.0) (struct) 1.0 1.0 0.0 null null null null)
      (`self.ResetWeapon`))))

(event `self.ResetWeapon`
  (goto _label :!via `Reset`))

(fn `UserConstructionScript`
  (`parent.UserConstructionScript`))